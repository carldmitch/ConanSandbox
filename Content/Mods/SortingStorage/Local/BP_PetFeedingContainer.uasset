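; Pet feeding container placeable from the SortingStorage mod that shows how full it is with a food plane and supplies a PetItemDistributor.
; On non-dedicated instances, BeginPlay creates an inventory client monitor so contents load without prior interaction.
; Item added and removed signals update the plane's height from the ratio of populated slots to capacity, hiding it when empty.
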(event `self.ReceiveBeginPlay`
  (bind _placeableinventory (`self.PlaceableInventory`))
  (`parent.ReceiveBeginPlay`)
  (if (not (`KismetSystemLibrary.IsDedicatedServer`))
    (`|ExecutionSequence`
      (:`then_0`
        ;[0.02499 0.09524 0.16] Make sure the the inventory is loaded even if it hasn't been interacted with.
        (if (not (`KismetSystemLibrary.IsDedicatedServer`))
          (bind _returnvalue (`|GenericCreateObject` "/Script/ConanSandbox.ItemInventoryClientMonitor" self))
          (`ItemInventoryClientMonitor.SetInventory` _returnvalue (`self.PlaceableInventory`))))
      (:`then_1`
        (add `ItemInventory.SignalItemAdded` _placeableinventory (delegate `SetFoodPlaneHeight`))
        (add `ItemInventory.SignalItemRemoved` _placeableinventory (delegate `SetFoodPlaneHeight`)))
      (:`then_2`
        ;[1 0.6413 0.1882] Set Z location of FoodPlane
        (`SceneComponent.K2_SetRelativeLocation` (`self.FoodPlane`) (`KismetMathLibrary.MakeVector` 0.0 0.0 (`KismetMathLibrary.Lerp` -35.0 15.0 (/ (`KismetMathLibrary.Conv_IntToDouble` (`ItemInventory.GetPopulatedItemCount` (`self.PlaceableInventory`) 0 -1)) (`KismetMathLibrary.Conv_IntToDouble` (`ItemInventory.MaxItemCount` (`self.PlaceableInventory`)))))) false false :!label _label)
        ;[1 0.6413 0.1882] Handle Visibility
        (if (== (`ItemInventory.GetPopulatedItemCount` (`self.PlaceableInventory`) 0 -1) 0)
          (`SceneComponent.SetVisibility` (`self.FoodPlane`) false false)
          (else
            (`SceneComponent.SetVisibility` (`self.FoodPlane`) true false)))))))

(event `SetFoodPlaneHeight`
  (params (index :type Integer) (item :type "GameItem Object Reference") (dstInventory :type "ItemInventory Object Reference") (dstIndex :type Integer))
  ;[1 0.6413 0.1882] Set Z location of FoodPlane
  (goto _label))

(fn `GetItemDistributor`
  (returns (ItemDistributor :type "/Game/Systems/Building/Placeables/ItemDistributor Object Reference"))
  (return (`self.PetItemDistributor`)))

(fn `UserConstructionScript`
  (`parent.UserConstructionScript`))