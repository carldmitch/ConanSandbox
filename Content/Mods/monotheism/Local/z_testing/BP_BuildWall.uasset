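; BP_BuildWall is a wall building-piece Blueprint in a mod's testing folder, with a placement-validation override.
; CanBePlaced calls the parent check and compares its result against Fail, but both branches return the parent's result and message unchanged.
; The construction script only calls its parent, and the event graph holds only disabled placeholder events, so the asset adds no behavior in these graphs.
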(fn `CanBePlaced`
  (params (AttachTo :type "BuildableBase Object Reference") (InstanceIndex :type Integer))
  (returns (FailedMessage :type String) (ReturnValue :type "ECanBePlacedResult Enum"))
  (bind (_failedmessage _returnvalue) (`parent.CanBePlaced` AttachTo InstanceIndex))
  (if (< (`KismetMathLibrary.Conv_ByteToInt` _returnvalue) (`KismetMathLibrary.Conv_ByteToInt` (enumliteral `ECanBePlacedResult` "Fail")))
    (return _failedmessage _returnvalue)
    (else
      (return _failedmessage _returnvalue))))

(fn `UserConstructionScript`
  (`parent.UserConstructionScript`))