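; Placeable legendary loot chest that opens only for players of at least level 60 carrying a key item, otherwise showing a HUD notification.
; Activation runs the parent interaction, deletes one key and sets HasBeenOpened, which lets later users in without a key, though any key they carry is still consumed.
; Inventory removal and stat-change signals recount the Legendaries templates and destroy the chest when none remain.
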(event `self.ItemInventoryReplicateToAll.SignalItemRemoved`
  (params (index :type Integer) (item :type "GameItem Object Reference") (dstInventory :type "ItemInventory Object Reference") (dstIndex :type Integer))
  (set `self.Counter` 0 :!label _label)
  (for _array_element (`self.Legendaries`)
    (bind _resourcecount (`/Game/Systems/MiscFunctions.GetCompleteResourceCount` null _array_element))
    (set `self.Counter` (+ _resourcecount (`self.Counter`))))
  (if (< (`self.Counter`) 1)
    (`self.K2_DestroyActor`)))

(event `self.ItemInventoryReplicateToAll.SignalItemAdded`
  (params (index :type Integer) (item :type "GameItem Object Reference") (srcInventory :type "ItemInventory Object Reference") (srcIndex :type Integer)))

(event `self.ItemInventoryReplicateToAll.SignalItemFloatStatChanged`
  (params (item :type "GameItem Object Reference") (statID :type "EItemFloatStatID Enum" :default "WeaponStaminaHeavyChargedRegenModifier") (statValue :type "Float (single-precision)") (deltaValue :type "Float (single-precision)"))
  (goto _label))

(event `self.ItemInventoryReplicateToAll.SignalItemIntStatChanged`
  (params (item :type "GameItem Object Reference") (statID :type "EItemIntStatID Enum" :default "MaxStackSize") (statValue :type Integer) (deltaValue :type Integer))
  (goto _label))

(event `InteractableInterface.InteractableActivate`
  (params (Component :type "PrimitiveComponent Object Reference") (Instigator :type "PlayerController Object Reference") (HitIndex :type Integer))
  (bind _returnvalue (`Controller.K2_GetPawn` Instigator))
  (bind _asconan_character (cast `ConanCharacter` _returnvalue :!pure true))
  (bind _asbase_player_char (cast `/Game/Characters/BasePlayerChar` _returnvalue))
  (if (< (`/Game/Systems/Progression/BP_ProgressionSystem.GetLevel` (`/Game/Characters/BasePlayerChar.BP_ProgressionSystem` _asbase_player_char)) 60)
    (`ConanCharacter.ClientHUDShowNotification` _asconan_character (`self.MustBeLevel60`) false)
    (else
      (bind _returnvalue_2 (`ConanCharacter.GetBackpackInventory` _asconan_character))
      (if (`ItemInventory.HasItemByTemplateID` _returnvalue_2 11073 1)
        (`parent.InteractableActivate` Component Instigator HitIndex :!label _label_2)
        (`ItemInventory.DeleteItemsByTemplate` _returnvalue_2 11073 1)
        (set `self.HasBeenOpened` true)
        (elif (`self.HasBeenOpened`)
          (goto _label_2)
          (else
            (`ConanCharacter.ClientHUDShowNotification` _asconan_character (`self.MustHaveKey`) false)))))))

(fn `UserConstructionScript`
  (`parent.UserConstructionScript`))