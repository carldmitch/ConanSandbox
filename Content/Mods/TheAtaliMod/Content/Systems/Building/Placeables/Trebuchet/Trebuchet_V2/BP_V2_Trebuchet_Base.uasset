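; Rotating base of the V2 trebuchet placeable, turned by characters pushing on its frame.
; Clockwise and counter-clockwise overlap boxes keep a net push count, which eases into rotation speed and stops faster when pushing ends.
; Tick runs only while turning, rotating the actor and counter-spinning its rollers.
; Each machine simulates locally; the server replicates the resting yaw on stop, and OnRep corrects only noticeable drift.
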(event `self.ReceiveBeginPlay`
  (`parent.ReceiveBeginPlay`)
  (set `self.ClientRotation` (`self.ServerRotation`))
  (`self.RotateBase`))

(event `self.ReceiveTick`
  (params (DeltaSeconds :type "Float (single-precision)"))
  ;[0.9019 1 0.377] OnTick - only ticks while it is actively rotating
  (`parent.ReceiveTick` DeltaSeconds)
  (set `self.CurrentSpeed` (`self.CalcNewRotationSpeed`))
  ;;[1 1 1] Check whether we're moving
  ;; slow enough to stop
  (if (`KismetMathLibrary.NearlyEqual_FloatFloat` (`self.CurrentSpeed`) 0.0 0.0001)
    (`self.SetActorTickEnabled` false)
    (if (`KismetSystemLibrary.IsServer`)
      (set `self.ServerRotation` (`self.ClientRotation`)))
    (else
      (set `self.ClientRotation` (+ (`self.ClientRotation`) (* (`GameplayStatics.GetWorldDeltaSeconds`) (`self.RotationDegreesPerSec`) (`self.CurrentSpeed`))))
      (`self.RotateBase`))))

(event `self.Push_CW1.OnComponentBeginOverlap`
  (params (OverlappedComponent :type "PrimitiveComponent Object Reference") (OtherActor :type "Actor Object Reference") (OtherComp :type "PrimitiveComponent Object Reference") (OtherBodyIndex :type Integer) (bFromSweep :type Boolean) (SweepResult :type "HitResult Structure (by ref)"))
  ;[1 1 1] Overlap boxes sense nr of people pushing the frame around
  (`/Engine/EditorBlueprintResources/StandardMacros.IncrementFloat` (`self.CurrentPushAmount`) :!label _label
    (:`  `
      (if (and (!= (`self.CurrentPushAmount`) 0.0) (not (`self.IsActorTickEnabled`))) :!label _label_2
        (`self.SetActorTickEnabled` true)))))

(event `self.Push_CW2.OnComponentBeginOverlap`
  (params (OverlappedComponent :type "PrimitiveComponent Object Reference") (OtherActor :type "Actor Object Reference") (OtherComp :type "PrimitiveComponent Object Reference") (OtherBodyIndex :type Integer) (bFromSweep :type Boolean) (SweepResult :type "HitResult Structure (by ref)"))
  ;[1 1 1] Overlap boxes sense nr of people pushing the frame around
  (goto _label))

(event `self.Push_CCW1.OnComponentEndOverlap`
  (params (OverlappedComponent :type "PrimitiveComponent Object Reference") (OtherActor :type "Actor Object Reference") (OtherComp :type "PrimitiveComponent Object Reference") (OtherBodyIndex :type Integer))
  ;[1 1 1] Overlap boxes sense nr of people pushing the frame around
  (goto _label))

(event `self.Push_CCW2.OnComponentEndOverlap`
  (params (OverlappedComponent :type "PrimitiveComponent Object Reference") (OtherActor :type "Actor Object Reference") (OtherComp :type "PrimitiveComponent Object Reference") (OtherBodyIndex :type Integer))
  ;[1 1 1] Overlap boxes sense nr of people pushing the frame around
  (goto _label))

(event `self.Push_CCW1.OnComponentBeginOverlap`
  (params (OverlappedComponent :type "PrimitiveComponent Object Reference") (OtherActor :type "Actor Object Reference") (OtherComp :type "PrimitiveComponent Object Reference") (OtherBodyIndex :type Integer) (bFromSweep :type Boolean) (SweepResult :type "HitResult Structure (by ref)"))
  ;[1 1 1] Overlap boxes sense nr of people pushing the frame around
  (`/Engine/EditorBlueprintResources/StandardMacros.DecrementFloat` (`self.CurrentPushAmount`) :!label _label_3
    (:`  `
      (goto _label_2))))

(event `self.Push_CCW2.OnComponentBeginOverlap`
  (params (OverlappedComponent :type "PrimitiveComponent Object Reference") (OtherActor :type "Actor Object Reference") (OtherComp :type "PrimitiveComponent Object Reference") (OtherBodyIndex :type Integer) (bFromSweep :type Boolean) (SweepResult :type "HitResult Structure (by ref)"))
  ;[1 1 1] Overlap boxes sense nr of people pushing the frame around
  (goto _label_3))

(event `self.Push_CW1.OnComponentEndOverlap`
  (params (OverlappedComponent :type "PrimitiveComponent Object Reference") (OtherActor :type "Actor Object Reference") (OtherComp :type "PrimitiveComponent Object Reference") (OtherBodyIndex :type Integer))
  ;[1 1 1] Overlap boxes sense nr of people pushing the frame around
  (goto _label_3))

(event `self.Push_CW2.OnComponentEndOverlap`
  (params (OverlappedComponent :type "PrimitiveComponent Object Reference") (OtherActor :type "Actor Object Reference") (OtherComp :type "PrimitiveComponent Object Reference") (OtherBodyIndex :type Integer))
  ;[1 1 1] Overlap boxes sense nr of people pushing the frame around
  (goto _label_3))

(fn `CalcNewRotationSpeed`
  (returns (OutputCurrentSpeed :type "Float (double-precision)"))
  (locals (LTargetSpeed :type "Float (double-precision)") (LInterpSpeed :type "Float (double-precision)" :default 0.1))
  (set `local.LTargetSpeed` (`self.CurrentPushAmount`))
  (if (== (`local.LTargetSpeed`) 0.0)
    (set `local.LInterpSpeed` 4.0)
    (else
      (set `local.LInterpSpeed` 0.2)))
  (return (`KismetMathLibrary.FInterpTo` (`self.CurrentSpeed`) (`local.LTargetSpeed`) (`GameplayStatics.GetWorldDeltaSeconds`) (`local.LInterpSpeed`))))

(fn `CanInteract`
  (params (Actor :type "Actor Object Reference"))
  (returns (CanInteract :type Boolean))
  (bind _aspawn (cast `Pawn` Actor)
    (:`then`
      (return (or (`self.IsOwner` _aspawn) (`ServerSettings.GetNoOwnership` (`|GetServerSettings`)))))
    (:`CastFailed`
      (return false))))

(fn `GetLoadRatio`
  (returns (Ratio :type "Float (double-precision)"))
  (return 0.0))

(fn `GetPayloadTemplateID`
  (returns (TemplateID :type Integer))
  (return 0))

(fn `OnRep_ServerRotation`
  (if (not (`KismetMathLibrary.NearlyEqual_FloatFloat` (`self.ServerRotation`) (`self.ClientRotation`) 2.0))
    (set `self.ClientRotation` (`self.ServerRotation`))))

(fn `RotateBase`
  (locals (LNewRollerRotation :type "Float (double-precision)"))
  (`self.K2_SetActorRelativeRotation` (`KismetMathLibrary.MakeRotator` 0.0 0.0 (`self.ClientRotation`)))
  (`SceneComponent.K2_SetRelativeRotation` (`self.Rollers_Scene`) (`KismetMathLibrary.MakeRotator` 0.0 0.0 (* (`self.ClientRotation`) 0.5)) false false)
  (set `local.LNewRollerRotation` (* -10.5 (`self.ClientRotation`)))
  (`SceneComponent.K2_SetRelativeRotation` (`self.Roller1`) (`KismetMathLibrary.MakeRotator` 0.0 (`local.LNewRollerRotation`)) false false)
  (`SceneComponent.K2_SetRelativeRotation` (`self.Roller2`) (`KismetMathLibrary.MakeRotator` 0.0 (`local.LNewRollerRotation`)) false false)
  (`SceneComponent.K2_SetRelativeRotation` (`self.Roller3`) (`KismetMathLibrary.MakeRotator` 0.0 (`local.LNewRollerRotation`)) false false)
  (`SceneComponent.K2_SetRelativeRotation` (`self.Roller4`) (`KismetMathLibrary.MakeRotator` 0.0 (`local.LNewRollerRotation`)) false false)
  (`SceneComponent.K2_SetRelativeRotation` (`self.Roller5`) (`KismetMathLibrary.MakeRotator` 0.0 (`local.LNewRollerRotation`)) false false)
  (`SceneComponent.K2_SetRelativeRotation` (`self.Roller6`) (`KismetMathLibrary.MakeRotator` 0.0 (`local.LNewRollerRotation`)) false false)
  (`SceneComponent.K2_SetRelativeRotation` (`self.Roller7`) (`KismetMathLibrary.MakeRotator` 0.0 (`local.LNewRollerRotation`)) false false)
  (`SceneComponent.K2_SetRelativeRotation` (`self.Roller8`) (`KismetMathLibrary.MakeRotator` 0.0 (`local.LNewRollerRotation`)) false false)
  (`SceneComponent.K2_SetRelativeRotation` (`self.Roller9`) (`KismetMathLibrary.MakeRotator` 0.0 (`local.LNewRollerRotation`)) false false)
  (`SceneComponent.K2_SetRelativeRotation` (`self.Roller10`) (`KismetMathLibrary.MakeRotator` 0.0 (`local.LNewRollerRotation`)) false false)
  (`SceneComponent.K2_SetRelativeRotation` (`self.Roller11`) (`KismetMathLibrary.MakeRotator` 0.0 (`local.LNewRollerRotation`)) false false)
  (`SceneComponent.K2_SetRelativeRotation` (`self.Roller12`) (`KismetMathLibrary.MakeRotator` 0.0 (`local.LNewRollerRotation`)) false false)
  (return))

(fn `UserConstructionScript`
  (`parent.UserConstructionScript`))