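; BP_PlaceableItemContainer is a placeable storage container that uses the "ContainerInfo" interaction UI module.
; On BeginPlay it spawns a game item from its source template to read the ItemContainerSize stat and size PlaceableInventory.
; If a journey event name is set, it binds to item-added signals and reports that event to the Exiles Journey component on the last activating instigator's pawn.
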(event `InteractableInterface.InteractableActivate`
  (params (Component :type "PrimitiveComponent Object Reference") (Instigator :type "PlayerController Object Reference") (HitIndex :type Integer))
  (`parent.InteractableActivate` Component Instigator HitIndex)
  (set `self.InteractingInstigator` Instigator))

(event `self.ReceiveBeginPlay`
  (`parent.ReceiveBeginPlay`)
  (bind _returnvalue (`GameItemSpawner.SpawnGameItem` (`self.SourceItemTemplateID`)))
  (`/Engine/EditorBlueprintResources/StandardMacros.IsValid` _returnvalue
    (:`Is Valid`
      (`ItemInventory.SetMaxItemCount` (`self.PlaceableInventory`) (`GameItem.GetIntStat` _returnvalue "ItemContainerSize"))
      (if (!= (`self.JourneyEventTriggerOnStoringItem`) "None")
        (add `ItemInventory.SignalItemAdded` (`self.PlaceableInventory`) (delegate `SignalItemAdded_Event_0`))))))

(event `SignalItemAdded_Event_0`
  (params (index :type Integer) (item :type "GameItem Object Reference") (srcInventory :type "ItemInventory Object Reference") (srcIndex :type Integer))
  (bind _interactinginstigator (`self.InteractingInstigator`))
  (bind _returnvalue (`Controller.K2_GetPawn` _interactinginstigator))
  (bind _returnvalue_2 (`self.GetComponentByClass` _returnvalue "/Game/Systems/Progression/BP_AC_ExilesJourney.BP_AC_ExilesJourney_C"))
  (`/Engine/EditorBlueprintResources/StandardMacros.IsValid` _interactinginstigator
    (:`Is Valid`
      (`/Engine/EditorBlueprintResources/StandardMacros.IsValid` _returnvalue_2
        (:`Is Valid`
          (`ExilesJourneyComponent.AddJourneyEvent` _returnvalue_2 (`self.JourneyEventTriggerOnStoringItem`) (`self.K2_GetActorLocation` _returnvalue)))))))

(fn `InteractableGetUIModuleName`
  (returns (ReturnValue :type Name))
  (return "ContainerInfo"))

(fn `UserConstructionScript`
  (`parent.UserConstructionScript`))