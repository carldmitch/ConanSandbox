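; Placeable respawn point that tries to bind itself as a spawn for the player who places it.
; Placement requires the parent checks plus a valid capsule-sized spot on one of the mesh's four sides.
; Each spot must pass an inside-collision test, a sphere sweep and a line-of-sight trace to the mesh center, ignoring blocker volumes and optionally brush buildables.
; The same search supplies the respawn transform and reports when all spots are blocked.
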(event `self.OnPlaced`
  (params (PlacedBy :type "ConanCharacter Object Reference"))
  (`parent.OnPlaced` PlacedBy)
  (`/Engine/EditorBlueprintResources/StandardMacros.IsValid` PlacedBy
    (:`Is Valid`
      (bind _asplayer_controller (cast `PlayerController` (`Pawn.GetController` PlacedBy)))
      (`/Game/Systems/Building/BuildingActorComponents/BP_BAC_SpawnPoints.TryBindSpawn` (`self.BP_BAC_SpawnPoints`) _asplayer_controller))))

(event `self.ReceiveDestroyed`
  (`self.OnBeingDestroyed`))

(fn `CanBePlaced`
  (params (AttachTo :type "BuildableBase Object Reference") (InstanceIndex :type Integer))
  (returns (FailedMessage :type String) (ReturnValue :type "ECanBePlacedResult Enum"))
  (bind (_failedmessage _returnvalue) (`parent.CanBePlaced` AttachTo InstanceIndex))
  (if (`|EnumEquality` _returnvalue "Success")
    (bind _foundvalidspawnpoint (`self.GetValidSpawnPoints` (`self.ShouldIgnoreBrushes`))) ; Passing None ActorToCheck, so that we check all actors.
    (return (select `bool` _foundvalidspawnpoint :`false` (`KismetTextLibrary.Conv_TextToString` (`self.Error_NoValidSpawnpoints`))) (select `bool` _foundvalidspawnpoint :`false` "Fail_InsideCollision" :`true` "Success" :!type "ECanBePlacedResult Enum"))
    (else
      (return _failedmessage _returnvalue))))

(fn `CheckForCollidingObjects`
  (params (CapsuleLocation :type "Vector Structure") (IgnoreBrushes :type Boolean))
  (returns (IsColliding :type Boolean))
  (locals (Local_CapsuleLocation :type "Vector Structure") (Local_ActorToCheck :type "Actor Object Reference") (Local_IgnoreBrushes :type Boolean))
  (bind (_capsulehalfheight _capsule_radius) (`self.GetSpawnPointCapsuleSize`))
  (`|ExecutionSequence`
    (:`then_0`
      ;[1 0.6413 0.1882] Initialize Local Variables
      (set `local.Local_CapsuleLocation` CapsuleLocation)
      (set `local.Local_IgnoreBrushes` IgnoreBrushes))
    (:`then_1`
      ;[1 0.6413 0.1882] Check if the capsule is entirely in collision. If it is, bypass other checks and return.
      (bind _returnvalue (`FuncomGenericLibrary.IsPointCompletelyInsideCollision` (+ (`local.Local_CapsuleLocation`) (`KismetMathLibrary.MakeVector` 0.0 0.0 (`self.GetSpawnPointCapsuleSize`))) (`|MakeArray` self :!type "Actor Object Reference") (not (`LoggerLibrary.IsSuppressed` "INFOL_INFO0" "Building"))))
      (if _returnvalue
        (return true)))
    (:`then_2`
      ;[1 0.6413 0.1882] Do Collision Trace
      (bind _outhits (`KismetSystemLibrary.SphereTraceMultiForObjects` :`Start` (+ (`local.Local_CapsuleLocation`) (`KismetMathLibrary.MakeVector` 0.0 0.0 (+ (`.Capsule Radius` (`self.GetSpawnPointCapsuleSize`)) 10.0))) :`End` (+ (`local.Local_CapsuleLocation`) (`KismetMathLibrary.MakeVector` 0.0 0.0 (- (* _capsulehalfheight 2.0) _capsule_radius))) :`Radius` (`.Capsule Radius` (`self.GetSpawnPointCapsuleSize`)) :`ObjectTypes` (`self.RespawnBlockingObjectTypes`) :`DrawDebugType` (select `bool` (`LoggerLibrary.IsSuppressed` "INFOL_INFO0" "Building") :`false` "ForDuration" :!type "EDrawDebugTrace Enum") :`DrawTime` 0.01))
      (bind _iscolliding (`self.CollidesWithSomething` _outhits (`local.Local_IgnoreBrushes`)))
      (return _iscolliding))))

(fn `CheckLineOfSightToPlaceable`
  (params (Start :type "Vector Structure") (IgnoreBrush :type Boolean))
  (returns (HasLineOfSight :type Boolean))
  (locals (LocalStart :type "Vector Structure") (LocalIgnoreBrush :type Boolean))
  (`|ExecutionSequence`
    (:`then_0`
      ;[1 0.6413 0.1882] Initialize Local Variables
      (set `local.LocalStart` Start)
      (set `local.LocalIgnoreBrush` IgnoreBrush))
    (:`then_1`
      (bind _outhits (`KismetSystemLibrary.LineTraceMultiForObjects` (`local.LocalStart`) (`self.GetCenterOfStaticMesh`) (`self.RespawnBlockingObjectTypes`) false (`|MakeArray` self :!type "Actor Object Reference") "None" true (struct :`R` 1.0 :`A` 1.0) (struct :`G` 1.0 :`A` 1.0) 0.01))
      (bind _iscolliding (`self.CollidesWithSomething` _outhits (`local.LocalIgnoreBrush`)))
      (return (not _iscolliding)))))

(fn `CollidesWithSomething`
  (params (`Hits results` :type "Array of HitResult Structure (by ref)") (LocalIgnoreBrushes :type Boolean))
  (returns (IsColliding :type Boolean))
  (for _array_element `Hits results`
    (bind (_bblockinghit _binitialoverlap _time _location _impactpoint _normal _impactnormal _physmat _hitactor) (`GameplayStatics.BreakHitResult` _array_element))
    (cast `/Game/Systems/Building/BuildingBlockerVolume` _hitactor
      (:`CastFailed`
        (bind _asbuildable_base (cast `BuildableBase` _hitactor)
          (:`then`
            (if (not (and (`BuildableBase.IsABrush` _asbuildable_base) LocalIgnoreBrushes))
              (return true)))
          (:`CastFailed`
            (return true))))))
  (return false))

(fn `GetCapsuleRespawnTransform`
  (returns (`Out Transform` :type "Transform Structure") (FoundValid :type Boolean))
  (bind (_foundvalidspawnpoint _spawnpoint) (`self.GetValidSpawnPoints` false))
  (return (`KismetMathLibrary.MakeTransform` _spawnpoint) _foundvalidspawnpoint))

(fn `GetCenterBottomOfStaticMesh`
  (returns (Center :type "Vector Structure"))
  (bind (_origin _boxextent) (`KismetSystemLibrary.GetComponentBounds` (`self.StaticMesh`)))
  (return (`KismetMathLibrary.MakeVector` (.x _origin) (.y _origin) (- (.z _origin) (.z _boxextent)))))

(fn `GetCenterOfStaticMesh`
  (returns (Center :type "Vector Structure"))
  (return (`KismetSystemLibrary.GetComponentBounds` (`self.StaticMesh`))))

(fn `GetIsActorOverlappingAllSpawnpoints`
  (returns (IsOverlappingAllSpawnpoints :type Boolean))
  (bind _foundvalidspawnpoint (`self.GetValidSpawnPoints` false))
  (return (not _foundvalidspawnpoint)))

(fn `GetSpawnPointCapsuleSize`
  (returns (CapsuleHalfHeight :type "Float (double-precision)") (`Capsule Radius` :type "Float (double-precision)"))
  (return 96.0 50.0))

(fn `GetSpawnPointsToCheck`
  (returns (`Out Spawnpoints` :type "Array of Vector Structure"))
  (bind _center (`self.GetCenterBottomOfStaticMesh`))
  (bind _center_2 (`self.GetCenterBottomOfStaticMesh`))
  (bind _staticmesh (`self.StaticMesh`))
  (bind _staticmesh_2 (`self.StaticMesh`))
  (bind _returnvalue (* (`SceneComponent.GetRightVector` _staticmesh_2) (+ (`.Capsule Radius` (`self.GetSpawnPointCapsuleSize`)) (.y (`.Max` (`StaticMeshComponent.GetLocalBounds` _staticmesh_2))))))
  (bind _returnvalue_2 (* (`SceneComponent.GetForwardVector` _staticmesh) (+ (`.Capsule Radius` (`self.GetSpawnPointCapsuleSize`)) (.x (`.Max` (`StaticMeshComponent.GetLocalBounds` _staticmesh))))))
  (return (`|MakeArray` (+ _center_2 _returnvalue) (- _center_2 _returnvalue) (+ _center _returnvalue_2) (- _center _returnvalue_2))))

(fn `GetValidSpawnPoints`
  (params (IgnoreBrushes :type Boolean))
  (returns (FoundValidSpawnPoint :type Boolean) (SpawnPoint :type "Vector Structure"))
  (locals (Local_ActorToCheck :type "Actor Object Reference") (Local_IgnoreBrushes :type Boolean))
  (`|ExecutionSequence`
    (:`then_0`
      ;[1 0.6413 0.1882] Initialize Local Variables
      (set `local.Local_IgnoreBrushes` IgnoreBrushes))
    (:`then_1`
      (bind _out_spawnpoints (`self.GetSpawnPointsToCheck`))
      (for _array_element _out_spawnpoints
        (bind _iscolliding (`self.CheckForCollidingObjects` _array_element (`local.Local_IgnoreBrushes`)))
        (if (not _iscolliding)
          (bind _returnvalue (+ _array_element (`KismetMathLibrary.MakeVector` 0.0 0.0 (`self.GetSpawnPointCapsuleSize`))))
          (if (`self.CheckLineOfSightToPlaceable` _returnvalue (`local.Local_IgnoreBrushes`))
            (return true _returnvalue))))
      (return false (0.0 0.0 0.0)))))

(fn `UserConstructionScript`)