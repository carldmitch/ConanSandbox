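; BP_CertainDeath is an admin-mod hazard that puts a configurable contact buff on any ConanCharacter inside its DamageContactBox.
; Server-only overlap events, skipped for brushes, track characters, applying the buff on entry and removing it on exit.
; A looping timer refreshes the buff on tracked characters, prunes invalid entries and is cleared when the last one leaves.
; The owner's controller, resolved from OwnerUniqueID, is passed as the buff's instigator.
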(event `self.DamageContactBox.OnComponentBeginOverlap`
  (params (OverlappedComponent :type "PrimitiveComponent Object Reference") (OtherActor :type "Actor Object Reference") (OtherComp :type "PrimitiveComponent Object Reference") (OtherBodyIndex :type Integer) (bFromSweep :type Boolean) (SweepResult :type "HitResult Structure (by ref)"))
  (if (`self.IsABrush`)
    _
    (elif (`KismetSystemLibrary.IsServer`)
      (bind _asconan_character (cast `ConanCharacter` OtherActor))
      (`KismetArrayLibrary.Array_AddUnique` (`self.OverlappingCharacters`) _asconan_character)
      (`self.ApplyOrRefreshBuff` _asconan_character)
      ;[0.02499 0.09524 0.16] Damage Tick. If the character has been in the array for too long, just remove it.
      (if (not (`KismetSystemLibrary.K2_IsTimerActiveHandle` (`self.DamageTickTimerHandle`)))
        (bind _returnvalue (`KismetSystemLibrary.K2_SetTimerDelegate` (delegate `RemoveCharacterFallback`) 0.8 true))
        (set `self.DamageTickTimerHandle` _returnvalue)))))

(event `self.DamageContactBox.OnComponentEndOverlap`
  (params (OverlappedComponent :type "PrimitiveComponent Object Reference") (OtherActor :type "Actor Object Reference") (OtherComp :type "PrimitiveComponent Object Reference") (OtherBodyIndex :type Integer))
  (bind _overlappingcharacters (`self.OverlappingCharacters`))
  (if (`self.IsABrush`)
    _
    (elif (`KismetSystemLibrary.IsServer`)
      (bind _asconan_character (cast `ConanCharacter` OtherActor))
      (`|ExecutionSequence`
        (:`then_0`
          (`KismetArrayLibrary.Array_RemoveItem` _overlappingcharacters _asconan_character)
          (if (<= (`KismetArrayLibrary.Array_Length` _overlappingcharacters) 0)
            ;[0.02499 0.09524 0.16] Damage Tick. If the character has been in the array for too long, just remove it.
            ;;[0.62 0 0] Stop timer if the Map is empty.
            (if (`KismetSystemLibrary.K2_IsTimerActiveHandle` (`self.DamageTickTimerHandle`))
              (`KismetSystemLibrary.K2_ClearAndInvalidateTimerHandle` (`self.DamageTickTimerHandle`)))))
        (:`then_1`
          ;;[0.62 0 0] Remove buff from the character when he leaves the overlapping area.
          (`/Game/Systems/Buffs/00_BP_AC_BuffSystem.RemoveBuff` (`KismetArrayLibrary.Array_Get` (`self.K2_GetComponentsByClass` _asconan_character "/Game/Systems/Buffs/00_BP_AC_BuffSystem.00_BP_AC_BuffSystem_C")) (`self.OnContactBuffToApply`)))))))

(event `RemoveCharacterFallback`
  ;[0.02499 0.09524 0.16] Damage Tick. If the character has been in the array for too long, just remove it.
  (for _array_element (`self.OverlappingCharacters`)
    ;;[1 0.6413 0.1882] Refresh the buff!
    (`/Engine/EditorBlueprintResources/StandardMacros.IsValid` _array_element
      (:`Is Valid`
        (`self.ApplyOrRefreshBuff` _array_element))
      (:`Is Not Valid`
        (`KismetArrayLibrary.Array_RemoveItem` (`self.OverlappingCharacters`) _array_element)))))

(fn `ApplyOrRefreshBuff`
  (params (ConanCharacter :type "Actor Object Reference"))
  (bind _returnvalue (`FuncomGenericLibrary.GetControllerFromUniqueId` self (`self.OwnerUniqueID`)))
  (`/Game/Systems/Buffs/00_BP_AC_BuffSystem.AddBuff` (`KismetArrayLibrary.Array_Get` (`self.K2_GetComponentsByClass` ConanCharacter "/Game/Systems/Buffs/00_BP_AC_BuffSystem.00_BP_AC_BuffSystem_C")) (`self.OnContactBuffToApply`) self 0 _returnvalue))

(fn `UserConstructionScript`
  (`parent.UserConstructionScript`))