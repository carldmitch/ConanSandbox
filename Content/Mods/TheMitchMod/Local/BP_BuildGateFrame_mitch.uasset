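; Modded gate frame building piece that overrides CanBePlaced to control where it can be built.
; Downward box traces require landscape or an allowed foundation mesh under the main checks, plus ground or foundation under both left and right sides.
; Foundations are recognized by matching instanced building meshes against hardcoded lists; missing support fails with a no-support error.
; Non-server instances skip these traces while loading, returning Success unless the parent check fails.
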(event `self.ReceiveBeginPlay`
  (`parent.ReceiveBeginPlay`))

(fn `CanBePlaced`
  (params (AttachTo :type "BuildableBase Object Reference") (InstanceIndex :type Integer))
  (returns (FailedMessage :type String) (ReturnValue :type "ECanBePlacedResult Enum"))
  (locals (HasFoundLandscape :type Boolean) (HasLeftSideSuccess :type Boolean) (HasRightSideSuccess :type Boolean))
  (bind _array (`|MakeArray` "/Game/Environment/Player_built/Meshes/SM_tier1_foundation.SM_tier1_foundation" "/Game/Environment/Player_built/Meshes/SM_tier2_foundation.SM_tier2_foundation" "/Game/Environment/Player_built/Meshes/SM_tier3_foundation.SM_tier3_foundation" "/Game/Environment/Player_built/Meshes/SM_tier1_sealing.SM_tier1_sealing" "/Game/Environment/Player_built/Meshes/SM_tier2_sealing.SM_tier2_sealing" "/Game/Environment/Player_built/Meshes/SM_tier3_sealing.SM_tier3_sealing" "/Game/Environment/Player_built/Meshes/SM_tier1_fence_foundation.SM_tier1_fence_foundation" "/Game/Environment/Player_built/Meshes/SM_tier2_fence_foundation.SM_tier2_fence_foundation" "/Game/Environment/Player_built/Meshes/SM_tier3_fence_foundation.SM_tier3_fence_foundation" "/Game/Environment/Player_built/Meshes/SM_tier2_fence_foundation_highlands.SM_tier2_fence_foundation_highlands" "/Game/Environment/Player_built/Meshes/SM_tier2_foundation_highlands.SM_tier2_foundation_highlands" "/Game/Environment/Player_built/Meshes/SM_tier2_ceiling_highlands.SM_tier2_ceiling_highlands" "/Game/Environment/Player_built/Meshes/SM_tier3_sealing_highlands.SM_tier3_sealing_highlands" "/Game/Environment/Player_built/Meshes/SM_tier3_fence_foundation_highlands.SM_tier3_fence_foundation_highlands" "/Game/Environment/Player_built/Meshes/SM_tier3_foundation_highlands.SM_tier3_foundation_highlands" "/Game/Environment/Player_built/Meshes/SM_tier1_foundation_triangle.SM_tier1_foundation_triangle" "/Game/Environment/Player_built/Meshes/SM_tier2_foundation_triangle.SM_tier2_foundation_triangle" "/Game/Environment/Player_built/Meshes/SM_tier2_foundation_triangle_highlands.SM_tier2_foundation_triangle_highlands" "/Game/Environment/Player_built/Meshes/SM_tier3_foundation_triangle.SM_tier3_foundation_triangle" "/Game/Environment/Player_built/Meshes/SM_tier3_foundation_triangle_highlands.SM_tier3_foundation_triangle_highlands" "/Game/Mods/TheMitchMod/drywood/T4/SM_004_fence_foundation.SM_004_fence_foundation" "/Game/Mods/TheMitchMod/brickwood/T2/SM_004_fence_foundation.SM_004_fence_foundation" "/Game/Mods/TheMitchMod/redclay/T2/SM_004_fence_foundation.SM_004_fence_foundation" :!type "StaticMesh Object Reference"))
  (bind _checkforlandscape (`self.CheckForLandscape`))
  (bind _checkforvalidbuildingsupport (`self.CheckForValidBuildingSupport`))
  (bind _rightsidecheck (`self.RightSideCheck`))
  (bind _leftsidecheck (`self.LeftSideCheck`))
  (bind _returnvalue (`SceneComponent.K2_GetComponentLocation` _rightsidecheck))
  (bind _returnvalue_2 (`SceneComponent.K2_GetComponentLocation` _checkforlandscape))
  (bind _returnvalue_3 (`SceneComponent.K2_GetComponentLocation` _checkforvalidbuildingsupport))
  (bind _returnvalue_4 (`SceneComponent.K2_GetComponentLocation` _leftsidecheck))
  (bind (_failedmessage _returnvalue_5) (`parent.CanBePlaced` AttachTo InstanceIndex))
  (if (`KismetSystemLibrary.IsServer`)
    (if (< (`KismetMathLibrary.Conv_ByteToInt` _returnvalue_5) (`KismetMathLibrary.Conv_ByteToInt` (enumliteral `ECanBePlacedResult` "Fail")))
      _
      (else
        (return _failedmessage _returnvalue_5)))
    (elif (`self.m_IsLoading`)
      (if (< (`KismetMathLibrary.Conv_ByteToInt` _returnvalue_5) (`KismetMathLibrary.Conv_ByteToInt` (enumliteral `ECanBePlacedResult` "Fail")))
        (return "" "Success")
        (else
          (return _failedmessage _returnvalue_5)))
      (else
        _)))
  (bind _outhits (`KismetSystemLibrary.BoxTraceMulti` (`KismetMathLibrary.MakeVector` (.x _returnvalue_2) (.y _returnvalue_2) (+ (.z _returnvalue_2) 128.0)) (`KismetMathLibrary.MakeVector` (.x _returnvalue_2) (.y _returnvalue_2) (- (.z _returnvalue_2) 32.0)) (`BoxComponent.BoxExtent` _checkforlandscape) (`SceneComponent.K2_GetComponentRotation` _checkforlandscape) "TraceTypeQuery1"))
  (bind _returnvalue_6 (`BuildableFunctionLibrary.HasStaticGroundInHitResults` _outhits))
  (set `local.HasFoundLandscape` _returnvalue_6)
  ;[1 0.04911 0] Build on top of foundations - remember to enable for triangles too
  (`KismetArrayLibrary.Array_Clear` (`self.FoundFoundation`))
  (bind _outhits_2 (`KismetSystemLibrary.BoxTraceMulti` (`KismetMathLibrary.MakeVector` (.x _returnvalue_3) (.y _returnvalue_3) (.z _returnvalue_3)) (`KismetMathLibrary.MakeVector` (.x _returnvalue_3) (.y _returnvalue_3) (- (.z _returnvalue_3) 32.0)) (`BoxComponent.BoxExtent` _checkforvalidbuildingsupport) (`SceneComponent.K2_GetComponentRotation` _checkforvalidbuildingsupport) "TraceTypeQuery3"))
  (for _array_element _outhits_2
    (bind _asinstanced_building_component (cast `InstancedBuildingComponent` (`.HitComponent` (`GameplayStatics.BreakHitResult` _array_element))))
    (`KismetArrayLibrary.Array_Add` (`self.FoundFoundation`) (`KismetArrayLibrary.Array_Contains` (`|MakeArray` "/Game/Environment/Player_built/Meshes/SM_tier1_foundation.SM_tier1_foundation" "/Game/Environment/Player_built/Meshes/SM_tier2_foundation.SM_tier2_foundation" "/Game/Environment/Player_built/Meshes/SM_tier3_foundation.SM_tier3_foundation" "/Game/Environment/Player_built/Meshes/SM_tier1_sealing.SM_tier1_sealing" "/Game/Environment/Player_built/Meshes/SM_tier2_sealing.SM_tier2_sealing" "/Game/Environment/Player_built/Meshes/SM_tier3_sealing.SM_tier3_sealing" "/Game/Environment/Player_built/Meshes/SM_tier1_fence_foundation.SM_tier1_fence_foundation" "/Game/Environment/Player_built/Meshes/SM_tier2_fence_foundation.SM_tier2_fence_foundation" "/Game/Environment/Player_built/Meshes/SM_tier3_fence_foundation.SM_tier3_fence_foundation" "/Game/Environment/Player_built/Meshes/SM_tier2_fence_foundation_highlands.SM_tier2_fence_foundation_highlands" "/Game/Environment/Player_built/Meshes/SM_tier2_foundation_highlands.SM_tier2_foundation_highlands" "/Game/Environment/Player_built/Meshes/SM_tier2_ceiling_highlands.SM_tier2_ceiling_highlands" "/Game/Environment/Player_built/Meshes/SM_tier3_sealing_highlands.SM_tier3_sealing_highlands" "/Game/Environment/Player_built/Meshes/SM_tier3_fence_foundation_highlands.SM_tier3_fence_foundation_highlands" "/Game/Environment/Player_built/Meshes/SM_tier3_foundation_highlands.SM_tier3_foundation_highlands" "/Game/Environment/Player_built/Meshes/SM_tier1_foundation_triangle.SM_tier1_foundation_triangle" "/Game/Environment/Player_built/Meshes/SM_tier2_foundation_triangle.SM_tier2_foundation_triangle" "/Game/Environment/Player_built/Meshes/SM_tier2_foundation_triangle_highlands.SM_tier2_foundation_triangle_highlands" "/Game/Environment/Player_built/Meshes/SM_tier3_foundation_triangle.SM_tier3_foundation_triangle" "/Game/Environment/Player_built/Meshes/SM_tier3_foundation_triangle_highlands.SM_tier3_foundation_triangle_highlands" "/Game/Mods/TheMitchMod/drywood/T4/SM_004_fence_foundation.SM_004_fence_foundation" "/Game/Mods/TheMitchMod/brickwood/T2/SM_004_fence_foundation.SM_004_fence_foundation" "/Game/Mods/TheMitchMod/redclay/T2/SM_004_fence_foundation.SM_004_fence_foundation" :!type "StaticMesh Object Reference") (`StaticMeshComponent.StaticMesh` _asinstanced_building_component))))
  ;[1 0.04911 0] LeftSide
  (bind _outhits_3 (`KismetSystemLibrary.BoxTraceMulti` (`KismetMathLibrary.MakeVector` (.x _returnvalue_4) (.y _returnvalue_4) (.z _returnvalue_4)) (`KismetMathLibrary.MakeVector` (.x _returnvalue_4) (.y _returnvalue_4) (- (.z _returnvalue_4) 32.0)) (`BoxComponent.BoxExtent` _leftsidecheck) (`SceneComponent.K2_GetComponentRotation` _leftsidecheck) "TraceTypeQuery1"))
  (bind _returnvalue_7 (`BuildableFunctionLibrary.HasStaticGroundInHitResults` _outhits_3))
  (bind _output_get (set `local.HasLeftSideSuccess` _returnvalue_7))
  (if (not _output_get)
    (for _array_element_2 _outhits_3
      (bind _asinstanced_building_component_2 (cast `InstancedBuildingComponent` (`.HitComponent` (`GameplayStatics.BreakHitResult` _array_element_2))))
      (if (`KismetArrayLibrary.Array_Contains` _array (`StaticMeshComponent.StaticMesh` _asinstanced_building_component_2))
        (set `local.HasLeftSideSuccess` true)
        (break))))
  ;[1 0.04911 0] Rightside
  (bind _outhits_4 (`KismetSystemLibrary.BoxTraceMulti` (`KismetMathLibrary.MakeVector` (.x _returnvalue) (.y _returnvalue) (.z _returnvalue)) (`KismetMathLibrary.MakeVector` (.x _returnvalue) (.y _returnvalue) (- (.z _returnvalue) 32.0)) (`BoxComponent.BoxExtent` _rightsidecheck) (`SceneComponent.K2_GetComponentRotation` _rightsidecheck) "TraceTypeQuery1"))
  (bind _returnvalue_8 (`BuildableFunctionLibrary.HasStaticGroundInHitResults` _outhits_4))
  (bind _output_get_2 (set `local.HasRightSideSuccess` _returnvalue_8))
  (if (not _output_get_2)
    (for _array_element_3 _outhits_4
      (bind _asinstanced_building_component_3 (cast `InstancedBuildingComponent` (`.HitComponent` (`GameplayStatics.BreakHitResult` _array_element_3))))
      (if (`KismetArrayLibrary.Array_Contains` _array (`StaticMeshComponent.StaticMesh` _asinstanced_building_component_3))
        (set `local.HasRightSideSuccess` true))))
  (if (and (or (`local.HasFoundLandscape`) (`KismetArrayLibrary.Array_Contains` (`self.FoundFoundation`) true)) (and (`local.HasLeftSideSuccess`) (`local.HasRightSideSuccess`)))
    (return _failedmessage _returnvalue_5)
    (else
      (return (`KismetTextLibrary.Conv_TextToString` (`self.Error_NoSupport`)) "Fail"))))

(fn `UserConstructionScript`
  (`parent.UserConstructionScript`))