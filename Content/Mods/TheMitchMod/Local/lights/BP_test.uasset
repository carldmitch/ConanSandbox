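; Placeable mod light that changes its point light colour and pyro particle effect according to the powder in its inventory.
; On BeginPlay, non-servers create an inventory client monitor; inventory receipt, item additions, removals and stat changes all rerun Update.
; Update checks a list of powder template IDs and calls SetFlame for each one present, so the last match wins.
; With no powder, only the light resets to white.
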(event `self.ReceiveBeginPlay`
  (bind _placeableinventory (`self.PlaceableInventory`))
  (if (not (`KismetSystemLibrary.IsServer`))
    (bind _returnvalue (`|GenericCreateObject` "/Script/ConanSandbox.ItemInventoryClientMonitor" self))
    (bind _output_get (set `self.InventoryMonitor` _returnvalue)))
  (`ItemInventoryClientMonitor.SetInventory` _output_get _placeableinventory)
  (add `ItemInventory.SignalInventoryRecivedOnClient` _placeableinventory (delegate `Update`))
  (`parent.ReceiveBeginPlay`))

(event `Update`
  (set `self.Resultcounter` 0 :!label _label)
  (set `self.PossibleResults` (`|MakeArray` 17030 17108 17114 17113 17093 17040 17112 17020))
  (for (_array_element _array_index) (`self.PossibleResults`)
    (if (`ItemInventory.HasItemByTemplateID` (`self.PlaceableInventory`) _array_element 1)
      (set `self.Resultcounter` 1)
      (bind _output_get (set `self.ArrayIndexHit` _array_index))
      (`self.SetFlame` _output_get)))
  (if (not (> (`self.Resultcounter`) 0))
    (`LightComponent.SetLightColor` (`self.PointLight_0`) (struct :`R` 1.0 :`G` 1.0 :`B` 1.0 :`A` 1.0) true)))

(event `self.PlaceableInventory.SignalItemRemoved`
  (params (index :type Integer) (item :type "GameItem Object Reference") (dstInventory :type "ItemInventory Object Reference") (dstIndex :type Integer))
  (goto _label))

(event `self.PlaceableInventory.SignalItemAdded`
  (params (index :type Integer) (item :type "GameItem Object Reference") (srcInventory :type "ItemInventory Object Reference") (srcIndex :type Integer))
  (goto _label))

(event `self.PlaceableInventory.SignalItemIntStatChanged`
  (params (item :type "GameItem Object Reference") (statID :type "EItemIntStatID Enum" :default "MaxStackSize") (statValue :type Integer) (deltaValue :type Integer))
  (goto _label))

(event `self.PlaceableInventory.SignalItemFloatStatChanged`
  (params (item :type "GameItem Object Reference") (statID :type "EItemFloatStatID Enum" :default "WeaponStaminaHeavyChargedRegenModifier") (statValue :type "Float (single-precision)") (deltaValue :type "Float (single-precision)"))
  (goto _label))

(fn `SetFlame`
  (params (index :type Integer))
  (bind _item (`KismetArrayLibrary.Array_Get` (`self.PossibleResults`) index))
  (if (== _item 17020)
    (`LightComponent.SetLightColor` (`self.PointLight_0`) (`self.Smokey_Light`) true)
    (`ParticleSystemComponent.SetTemplate` (`self.ParticleSystem1`) "/Game/Mods/TheMitchMod/lights/grey/P_pyro_grey.P_pyro_grey")
    (elif (== _item 17040)
      (`LightComponent.SetLightColor` (`self.PointLight_0`) (`self.Ruby_Light`) true)
      (`ParticleSystemComponent.SetTemplate` (`self.ParticleSystem1`) "/Game/Mods/TheMitchMod/lights/red/P_pyro_red.P_pyro_red")
      (elif (== _item 17112)
        (`LightComponent.SetLightColor` (`self.PointLight_0`) (`self.Blue_Light`) true)
        (`ParticleSystemComponent.SetTemplate` (`self.ParticleSystem1`) "/Game/Mods/TheMitchMod/lights/blue/P_pyro_blue.P_pyro_blue")
        (elif (== _item 17113)
          (`LightComponent.SetLightColor` (`self.PointLight_0`) (`self.Purple_Light`) true)
          (`ParticleSystemComponent.SetTemplate` (`self.ParticleSystem1`) "/Game/Mods/TheMitchMod/lights/purple/P_pyro_purple.P_pyro_purple")
          (elif (== _item 17114)
            (`LightComponent.SetLightColor` (`self.PointLight_0`) (`self.Green_Light`) true)
            (`ParticleSystemComponent.SetTemplate` (`self.ParticleSystem1`) "/Game/Mods/TheMitchMod/lights/green/P_pyro_green.P_pyro_green")
            (elif (== _item 17108)
              (`LightComponent.SetLightColor` (`self.PointLight_0`) (`self.Gold_Light`) true)
              (`ParticleSystemComponent.SetTemplate` (`self.ParticleSystem1`) "/Game/Mods/TheMitchMod/lights/gold/P_pyro_gold.P_pyro_gold")
              (elif (== _item 17030)
                (`LightComponent.SetLightColor` (`self.PointLight_0`) (`self.Teal_Light`) true)
                (`ParticleSystemComponent.SetTemplate` (`self.ParticleSystem1`) "/Game/Mods/TheMitchMod/lights/teal/P_pyro_teal.P_pyro_teal")
                (elif (== _item 17093)
                  (`LightComponent.SetLightColor` (`self.PointLight_0`) (`self.Pink_Light`) true)
                  (`ParticleSystemComponent.SetTemplate` (`self.ParticleSystem1`) "/Game/Mods/TheMitchMod/lights/pink/P_pyro_pink.P_pyro_pink"))))))))))

(fn `UserConstructionScript`
  (`parent.UserConstructionScript`))