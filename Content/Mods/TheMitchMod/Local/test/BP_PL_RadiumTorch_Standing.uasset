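; Placeable standing radium torch whose point light color and gem mesh follow the dye stored in its inventory.
; BeginPlay creates a client inventory monitor on non-servers; inventory receipt, item changes and stat changes all rerun the dye check.
; The check scans a fixed list of dye template IDs, with the last match winning, and MakeLight applies that color and mesh.
; Without dye, it falls back to white.
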(event `self.ReceiveBeginPlay`
  (bind _placeableinventory (`self.PlaceableInventory`))
  (if (not (`KismetSystemLibrary.IsServer`))
    (bind _returnvalue (`|GenericCreateObject` "/Script/ConanSandbox.ItemInventoryClientMonitor" self))
    (bind _output_get (set `self.InventoryMonitor` _returnvalue)))
  (`ItemInventoryClientMonitor.SetInventory` _output_get _placeableinventory)
  (add `ItemInventory.SignalInventoryRecivedOnClient` _placeableinventory (delegate `Update`))
  (`parent.ReceiveBeginPlay`))

(event `Update`
  (set `self.Resultcounter` 0 :!label _label)
  (set `self.PossibleResults` (`|MakeArray` 17010 17020 17030 17040 17050 17060 17070 17080 17090 17093))
  (for (_array_element _array_index) (`self.PossibleResults`)
    (if (`ItemInventory.HasItemByTemplateID` (`self.PlaceableInventory`) _array_element 1)
      (set `self.Resultcounter` 1)
      (bind _output_get (set `self.ArrayIndexHit` _array_index))
      (`self.MakeLight` _output_get)))
  (if (not (> (`self.Resultcounter`) 0))
    (`LightComponent.SetLightColor` (`self.PointLight`) (struct :`R` 1.0 :`G` 1.0 :`B` 1.0 :`A` 1.0) true)
    (`StaticMeshComponent.SetStaticMesh` (`self.Gem`) "/Game/Items/Placeables/Meshes/SM_white_radium_gem.SM_white_radium_gem")))

(event `self.PlaceableInventory.SignalItemRemoved`
  (params (index :type Integer) (item :type "GameItem Object Reference") (dstInventory :type "ItemInventory Object Reference") (dstIndex :type Integer))
  (goto _label))

(event `self.PlaceableInventory.SignalItemAdded`
  (params (index :type Integer) (item :type "GameItem Object Reference") (srcInventory :type "ItemInventory Object Reference") (srcIndex :type Integer))
  (goto _label))

(event `self.PlaceableInventory.SignalItemIntStatChanged`
  (params (item :type "GameItem Object Reference") (statID :type "EItemIntStatID Enum" :default "MaxStackSize") (statValue :type Integer) (deltaValue :type Integer))
  (goto _label))

(event `self.PlaceableInventory.SignalItemFloatStatChanged`
  (params (item :type "GameItem Object Reference") (statID :type "EItemFloatStatID Enum" :default "WeaponStaminaHeavyChargedRegenModifier") (statValue :type "Float (single-precision)") (deltaValue :type "Float (single-precision)"))
  (goto _label))

(fn `MakeLight`
  (params (Index :type Integer))
  (bind _item (`KismetArrayLibrary.Array_Get` (`self.PossibleResults`) Index))
  (if (== _item 17010)
    (`LightComponent.SetLightColor` (`self.PointLight`) (`self.Light_Brown`) true)
    (`StaticMeshComponent.SetStaticMesh` (`self.Gem`) "/Game/Items/Placeables/Meshes/SM_orange_radium_gem.SM_orange_radium_gem")
    (elif (== _item 17020)
      (`LightComponent.SetLightColor` (`self.PointLight`) (`self.Light_Grey`) true)
      (`StaticMeshComponent.SetStaticMesh` (`self.Gem`) "/Game/Items/Placeables/Meshes/SM_white_radium_gem.SM_white_radium_gem")
      (elif (== _item 17030)
        (`LightComponent.SetLightColor` (`self.PointLight`) (`self.Light_Cyan`) true)
        (`StaticMeshComponent.SetStaticMesh` (`self.Gem`) "/Game/Items/Placeables/Meshes/SM_cyan_radium_gem.SM_cyan_radium_gem")
        (elif (== _item 17040)
          (`LightComponent.SetLightColor` (`self.PointLight`) (`self.Light_Red`) true)
          (`StaticMeshComponent.SetStaticMesh` (`self.Gem`) "/Game/Items/Placeables/Meshes/SM_red_radium_gem.SM_red_radium_gem")
          (elif (== _item 17050)
            (`LightComponent.SetLightColor` (`self.PointLight`) (`self.Light_Blue`) true)
            (`StaticMeshComponent.SetStaticMesh` (`self.Gem`) "/Game/Items/Placeables/Meshes/SM_blue_radium_gem.SM_blue_radium_gem")
            (elif (== _item 17060)
              (`LightComponent.SetLightColor` (`self.PointLight`) (`self.Light_Green`) true)
              (`StaticMeshComponent.SetStaticMesh` (`self.Gem`) "/Game/Items/Placeables/Meshes/SM_green_radium_gem.SM_green_radium_gem")
              (elif (== _item 17070)
                (`LightComponent.SetLightColor` (`self.PointLight`) (`self.Light_Yellow`) true)
                (`StaticMeshComponent.SetStaticMesh` (`self.Gem`) "/Game/Items/Placeables/Meshes/SM_yellow_radium_gem.SM_yellow_radium_gem")
                (elif (== _item 17080)
                  (`LightComponent.SetLightColor` (`self.PointLight`) (`self.Light_Purple`) true)
                  (`StaticMeshComponent.SetStaticMesh` (`self.Gem`) "/Game/Items/Placeables/Meshes/SM_purple_radium_gem.SM_purple_radium_gem")
                  (elif (== _item 17090)
                    (`LightComponent.SetLightColor` (`self.PointLight`) (`self.Light_Orange`) true)
                    (`StaticMeshComponent.SetStaticMesh` (`self.Gem`) "/Game/Items/Placeables/Meshes/SM_orange_radium_gem.SM_orange_radium_gem")
                    (elif (== _item 17093)
                      (`LightComponent.SetLightColor` (`self.PointLight`) (`self.Light_Magenta`) true)
                      (`StaticMeshComponent.SetStaticMesh` (`self.Gem`) "/Game/Items/Placeables/Meshes/SM_magenta_radium_gem.SM_magenta_radium_gem"))))))))))))

(fn `UserConstructionScript`
  (`parent.UserConstructionScript`))