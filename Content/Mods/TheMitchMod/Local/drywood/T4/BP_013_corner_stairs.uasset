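; Building-piece Blueprint for drywood T4 corner stairs that adds a placement check against stacking on existing stairs.
; CanBePlaced runs the parent check, then box-traces a short distance down from StairCheckerBox on the Visibility channel.
; Hit instanced building components have their meshes compared to a hardcoded list of tier 1–3 stair meshes.
; A match returns an overlap failure with a stair-specific error; otherwise the parent's result stands.
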(fn `CanBePlaced`
  (params (AttachTo :type "BuildableBase Object Reference") (InstanceIndex :type Integer))
  (returns (FailedMessage :type String) (ReturnValue :type "ECanBePlacedResult Enum"))
  (bind _staircheckerbox (`self.StairCheckerBox`))
  (bind _returnvalue (+ (`SceneComponent.K2_GetComponentLocation` _staircheckerbox) (`SceneComponent.RelativeLocation` _staircheckerbox)))
  (bind (_failedmessage _returnvalue_2) (`parent.CanBePlaced` AttachTo InstanceIndex))
  ;[1 1 1] Use StairCheckerBox to check for stairs underneath
  (`KismetArrayLibrary.Array_Clear` (`self.IsOverlappingStairs`))
  (bind _outhits (`KismetSystemLibrary.BoxTraceMulti` _returnvalue (- _returnvalue (0.0 0.0 16.0)) (`BoxComponent.BoxExtent` _staircheckerbox) (`SceneComponent.K2_GetComponentRotation` _staircheckerbox) "TraceTypeQuery1"))
  (for _array_element _outhits
    (bind _asinstanced_building_component (cast `InstancedBuildingComponent` (`.HitComponent` (`GameplayStatics.BreakHitResult` _array_element))))
    (`KismetArrayLibrary.Array_Add` (`self.IsOverlappingStairs`) (`KismetArrayLibrary.Array_Contains` (`|MakeArray` "/Game/Environment/Player_built/Meshes/SM_tier1_stair_256.SM_tier1_stair_256" "/Game/Environment/Player_built/Meshes/SM_tier2_stair_256.SM_tier2_stair_256" "/Game/Environment/Player_built/Meshes/SM_tier3_stair_256.SM_tier3_stair_256" "/Game/Environment/Player_built/Meshes/SM_tier2_stair_256_highlands.SM_tier2_stair_256_highlands" "/Game/Environment/Player_built/Meshes/SM_tier3_stair_256_highlands.SM_tier3_stair_256_highlands" :!type "StaticMesh Object Reference") (`StaticMeshComponent.StaticMesh` _asinstanced_building_component))))
  (if (`KismetArrayLibrary.Array_Contains` (`self.IsOverlappingStairs`) true)
    (return (`KismetTextLibrary.Conv_TextToString` (`self.Error_StairHittingStair`)) "Fail_Overlaps")
    (else
      (return _failedmessage _returnvalue_2))))

(fn `UserConstructionScript`
  (`parent.UserConstructionScript`))